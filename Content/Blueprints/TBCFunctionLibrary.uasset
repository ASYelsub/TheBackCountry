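; TBCFunctionLibrary is a Blueprint function library of global getters for the TBC game's HUD, UI, game state, Wolf, Crocodile and Pig clans, and selected creature.
; Base getters cast player 0's HUD to TBCHud and the game state to TBCGameState, and the other getters chain from them.
; Enum switches resolve a clan, its resource amount (Population, Food, Influence, Piety, Drama), or its resource bar widget.
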(fn `GetTBCClan`
  (params (Clan :type "/Game/Blueprints/Creatures/CreatureTypes Enum" :default "NewEnumerator0"))
  (returns (TBCClan :type "/Game/Blueprints/TBCClan Object Reference"))
  (switch `/Game/Blueprints/Creatures/CreatureTypes` Clan
    (:`NewEnumerator0`
      (return (`self.GetTBCWolfClan` null)))
    (:`NewEnumerator1`
      (return (`self.GetTBCCrocClan` null)))
    (:`NewEnumerator10`
      (return (`self.GetTBCPigClan ` null)))))

(fn `GetTBCCrocClan`
  (returns (CrocClan :type "/Game/Blueprints/TBCClan Object Reference"))
  (return (`/Game/Blueprints/TBCGameState.CrocClan` (`self.GetTBCGameState` null))))

(fn `GetTBCCurrentClan`
  (returns (CurrentClan :type "/Game/Blueprints/TBCClan Object Reference"))
  (return (`/Game/Blueprints/TBCGameState.CurrentClan` (`self.GetTBCGameState` null))))

(fn `GetTBCCurrentCreature`
  (returns (CurrentCreature :type "/Game/Blueprints/Creatures/CreatureBase Object Reference"))
  (return (`/Game/Blueprints/TBCGameState.SelectedCreature` (`self.GetTBCGameState` null))))

(fn `GetTBCGameState`
  (returns (GameState :type "/Game/Blueprints/TBCGameState Object Reference"))
  (bind _astbcgame_state (cast `/Game/Blueprints/TBCGameState` (`GameplayStatics.GetGameState` null)))
  (return _astbcgame_state))

(fn `GetTBCHud`
  (returns (TBCHud :type "/Game/Blueprints/Widgets/TBCHud Object Reference"))
  (bind _astbchud (cast `/Game/Blueprints/Widgets/TBCHud` (`PlayerController.GetHUD` (`GameplayStatics.GetPlayerController` null))))
  (return _astbchud))

(fn `GetTBCPigClan `
  (returns (PigClan :type "/Game/Blueprints/TBCClan Object Reference"))
  (return (`/Game/Blueprints/TBCGameState.PigClan` (`self.GetTBCGameState` null))))

(fn `GetTBCResourceAmount`
  (params (Clan :type "/Game/Blueprints/Creatures/CreatureTypes Enum" :default "NewEnumerator0") (ResourceType :type "/Game/Blueprints/ResourceTypes Enum" :default "NewEnumerator0"))
  (returns (Amount :type "Float (double-precision)"))
  (bind _tbcclan (`self.GetTBCClan` Clan))
  (switch `/Game/Blueprints/ResourceTypes` ResourceType
    (:`NewEnumerator0`
      (return (`/Game/Blueprints/TBCClan.Population` _tbcclan)))
    (:`NewEnumerator1`
      (return (`/Game/Blueprints/TBCClan.Food` _tbcclan)))
    (:`NewEnumerator2`
      (return (`/Game/Blueprints/TBCClan.Influence` _tbcclan)))
    (:`NewEnumerator3`
      (return (`/Game/Blueprints/TBCClan.Piety` _tbcclan)))
    (:`NewEnumerator4`
      (return (`/Game/Blueprints/TBCClan.Drama` _tbcclan)))))

(fn `GetTBCResourceBar`
  (params (CreatureType :type "/Game/Blueprints/Creatures/CreatureTypes Enum" :default "NewEnumerator0"))
  (returns (ResourceBar :type "/Game/Blueprints/Widgets/ResourceBar/TBCResourceBar Object Reference"))
  (bind _tbcresourcebarsparent (`self.GetTBCResourceBarsParent` null))
  (switch `/Game/Blueprints/Creatures/CreatureTypes` CreatureType
    (:`NewEnumerator0`
      (return (`/Game/Blueprints/Widgets/ResourceBar/TBCResourceBarsParent.WolfResourceBar` _tbcresourcebarsparent)))
    (:`NewEnumerator1`
      (return (`/Game/Blueprints/Widgets/ResourceBar/TBCResourceBarsParent.CrocResourceBar` _tbcresourcebarsparent)))
    (:`NewEnumerator10`
      (return (`/Game/Blueprints/Widgets/ResourceBar/TBCResourceBarsParent.PigResourceBar` _tbcresourcebarsparent)))))

(fn `GetTBCResourceBarsParent`
  (returns (TBCResourceBarsParent :type "/Game/Blueprints/Widgets/ResourceBar/TBCResourceBarsParent Object Reference"))
  (return (`/Game/Blueprints/Widgets/TBCUI.TBCResourceBarsParent` (`self.GetTBCUI` null))))

(fn `GetTBCUI`
  (returns (TBCUI :type "/Game/Blueprints/Widgets/TBCUI Object Reference"))
  (return (`/Game/Blueprints/Widgets/TBCHud.TBCUI` (`self.GetTBCHud` null))))

(fn `GetTBCWolfClan`
  (returns (WolfClan :type "/Game/Blueprints/TBCClan Object Reference"))
  (return (`/Game/Blueprints/TBCGameState.WolfClan` (`self.GetTBCGameState` null))))