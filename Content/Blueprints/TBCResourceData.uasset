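; TBCResourceData holds the display data for a clan's resources: Population, Food, Influence, Piety and Drama.
; On BeginPlay it fills ResourceNonModifiableStructs with a fixed tooltip title, description and icon for each resource.
; GetResourceAmount takes a resource type and creature type but only begins a switch on creature type, with no branches implemented.
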(event `self.ReceiveBeginPlay`
  (`self.SetResourceNonModifyStructs`))

(event `SetResourceNonModifyStructs`
  (bind _resourcenonmodifiablestructs (`self.ResourceNonModifiableStructs`))
  (`KismetArrayLibrary.Array_Add` _resourcenonmodifiablestructs (make `/Game/Blueprints/Widgets/ResourceBar/TBCResourceStructNonModify` "Population" "Amount of creatures in clan." "/Game/Blueprints/Widgets/ResourceBar/noun-population-2654135.noun-population-2654135"))
  (`KismetArrayLibrary.Array_Add` _resourcenonmodifiablestructs (make `/Game/Blueprints/Widgets/ResourceBar/TBCResourceStructNonModify` "Food" "Amount of food for clan." "/Game/Blueprints/Widgets/ResourceBar/noun-food-750655.noun-food-750655"))
  (`KismetArrayLibrary.Array_Add` _resourcenonmodifiablestructs (make `/Game/Blueprints/Widgets/ResourceBar/TBCResourceStructNonModify` "Influence" "Power of clan amongst others." "/Game/Blueprints/Widgets/ResourceBar/noun-influence-855684_1_.noun-influence-855684_1_"))
  (`KismetArrayLibrary.Array_Add` _resourcenonmodifiablestructs (make `/Game/Blueprints/Widgets/ResourceBar/TBCResourceStructNonModify` "Piety" "Clan's connection to player." "/Game/Blueprints/Widgets/ResourceBar/noun-religion-3817675.noun-religion-3817675"))
  (`KismetArrayLibrary.Array_Add` _resourcenonmodifiablestructs (make `/Game/Blueprints/Widgets/ResourceBar/TBCResourceStructNonModify` "Drama" "Earned drama for big buys." "/Game/Blueprints/Widgets/ResourceBar/noun-drama-2036471.noun-drama-2036471")))

(event `GetResourceAmount`
  (params (ResourceType :type "/Game/Blueprints/ResourceTypes Enum" :default "NewEnumerator0") (CreatureType :type "/Game/Blueprints/Creatures/CreatureTypes Enum" :default "NewEnumerator0"))
  (switch `/Game/Blueprints/Creatures/CreatureTypes` CreatureType))