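; Base creature Blueprint for a selectable AI animal with health, hunger and energy, with wolf animations as placeholders for child classes to override.
; Self-rescheduling Delay loops update the stats, and DecideNextAction picks flee, eat, sleep at home or roam.
; Eating requires a downward trace onto certain surface types; projectile hits cause fleeing or death and despawn.
; Hover shows the name label, and clicking selects the creature to feed the HUD each Tick.
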(event `self.ReceiveBeginPlay`
  (set `self.CursorStatus` "NewEnumerator0")
  (set `self.CurrentActivity` "NewEnumerator0")
  (bind _astbcplayer_controller (cast `/Game/Blueprints/TBCPlayerController` (`GameplayStatics.GetPlayerController` 0)))
  (set `self.PlayerCamera` (`/Game/Blueprints/TBCPlayerController.PlayerCamera` _astbcplayer_controller))
  (`self.SetText`)
  (`self.DrainEnergy`)
  (`self.Drain Hunger`)
  (`self.Decide Next Action` true)
  (`SceneComponent.SetVisibility` (`self.CreatureName`) false false :!label _label))

(event `self.ReceiveTick`
  (params (DeltaSeconds :type "Float (single-precision)"))
  (if (`self.IsSelectedCreature?`)
    (`self.New Creature UI`)))

(event `self.Mesh.OnEndCursorOver`
  (params (TouchedComponent :type "PrimitiveComponent Object Reference"))
  (set `self.CursorStatus` "NewEnumerator0")
  (goto _label))

(event `self.Mesh.OnClicked`
  (params (TouchedComponent :type "PrimitiveComponent Object Reference") (ButtonPressed :type "Key Structure"))
  (set `self.CursorStatus` "NewEnumerator2")
  (`self.SelectCreature`)
  (`SceneComponent.SetVisibility` (`self.CreatureName`) true false :!label _label_2))

(event `Go Home`
  ;[1 1 1] Go Home (and sleep)
  (set `self.CurrentActivity` "NewEnumerator4")
  (`|AIMoveTo` self (`self.HomeLocation`) null
    (:`OnSuccess`
      (`KismetSystemLibrary.PrintString` "success")
      (if (`self.IsTired?`)
        (`self.Rest`)
        (`self.RegainEnergy`)
        (else
          (`self.Decide Next Action` false))))
    (:`OnFail`
      (`KismetSystemLibrary.PrintString` "fail"))))

(event `self.Mesh.OnBeginCursorOver`
  (params (TouchedComponent :type "PrimitiveComponent Object Reference"))
  (set `self.CursorStatus` "NewEnumerator1")
  (goto _label_2))

(event `self.Mesh.OnReleased`
  (params (TouchedComponent :type "PrimitiveComponent Object Reference") (ButtonReleased :type "Key Structure"))
  (set `self.CursorStatus` "NewEnumerator1")
  (goto _label_2))

(event `Rest`
  ;[1 1 1] SleepingAnim - This function should be overriden in children classes
  (set `self.CurrentActivity` "NewEnumerator5")
  (`MovementComponent.StopMovementImmediately` (`self.CharacterMovement`))
  (`self.PlayAnimation` null)
  (`KismetSystemLibrary.Delay` 0.99)
  (`self.PlayAnimation` null true)
  (`KismetSystemLibrary.Delay` (`KismetMathLibrary.Conv_IntToDouble` (`KismetMathLibrary.RandomIntegerInRange` 50 120)))
  (`self.PlayAnimation` null)
  (`KismetSystemLibrary.Delay` 0.99)
  (`self.StopAnimation`)
  (set `self.IsTired?` false)
  (`self.DrainEnergy`)
  (`self.Decide Next Action` false))

(event `Decide Next Action`
  (params (`SkipDelay?` :type Boolean))
  ;[1 1 1] AI Decision Tree
  (if (not `SkipDelay?`)
    (`KismetSystemLibrary.Delay` (`KismetMathLibrary.Conv_IntToDouble` (`KismetMathLibrary.RandomIntegerInRange` 1 5))))
  (if (`self.ShouldRun?`)
    (`self.RunAway`)
    (elif (`self.IsHungry?`)
      (`self.Eat`)
      (elif (`self.IsTired?`)
        (`self.Go Home`)
        (else
          (`self.Random Roam`)
          (`self.Regen Health`))))))

(event `DrainEnergy`
  ;[1 1 1] Drain Energy, normal = 125 seconds
  (if (not (`self.IsTired?`))
    (bind _output_get (set `self.Energy` (`KismetMathLibrary.Clamp` (- (`self.Energy`) (`self.EnergyDrain`)) 0 (`self.MaxEnergy`))))
    (if (== _output_get 0)
      (set `self.IsTired?` true)
      (`self.Decide Next Action` false)
      (else
        (`KismetSystemLibrary.Delay` 1.0)
        (`self.DrainEnergy`)))))

(event `Random Roam`
  ;[1 1 1] Random Roam
  (set `self.CurrentActivity` "NewEnumerator1")
  (set `CharacterMovementComponent.MaxWalkSpeed` 150.0 (`self.CharacterMovement`))
  (`|AIMoveTo` self (`NavigationSystemV1.K2_GetRandomReachablePointInRadius` (`self.K2_GetActorLocation`) 1500.0 null null) null
    (:`OnSuccess`
      (`self.Decide Next Action` self false))))

(event `RegainEnergy`
  ;[1 1 1] Regain Energy - takes 50 seconds
  (if (`self.IsTired?`)
    (bind _output_get (set `self.Energy` (`KismetMathLibrary.Clamp` (+ (`self.Energy`) (`self.EnergyGain`)) 0 (`self.MaxEnergy`))))
    (if (not (== _output_get (`self.MaxEnergy`)))
      (`KismetSystemLibrary.Delay` 1.0)
      (`self.RegainEnergy`))))

(event `RunAway`
  ;[1 1 1] Run Away
  (set `self.CurrentActivity` "NewEnumerator2")
  (set `CharacterMovementComponent.MaxWalkSpeed` 600.0 (`self.CharacterMovement`))
  (`|AIMoveTo` self (`NavigationSystemV1.K2_GetRandomReachablePointInRadius` (`self.K2_GetActorLocation`) (`KismetMathLibrary.RandomFloatInRange` 20000.0 30000.0) null null) null
    (:`OnSuccess`
      (set `self.ShouldRun?` false)
      (`self.Decide Next Action` true))))

(event `Eat`
  (bind _mesh (`self.Mesh`))
  ;[1 1 1] Eat Animation
  (bind _caneat_ (`self.CanEat`)
    (:`Out`
      (if _caneat_
        (set `self.CurrentActivity` "NewEnumerator3")
        (`MovementComponent.StopMovementImmediately` (`self.CharacterMovement`))
        ;;[1 1 1] These parts should be overriden by child classes to fit animations available
        (`self.Add Hunger`)
        (`SkeletalMeshComponent.PlayAnimation` _mesh "/Game/Blueprints/Creatures/Wolf/Animations/ANIM_Wolf_Bite.ANIM_Wolf_Bite" false)
        (`KismetSystemLibrary.Delay` 1.0)
        (`SkeletalMeshComponent.PlayAnimation` _mesh "/Game/Blueprints/Creatures/Wolf/Animations/ANIM_Wolf_Bite.ANIM_Wolf_Bite" true)
        (`KismetSystemLibrary.Delay` (`KismetMathLibrary.Conv_IntToDouble` (`KismetMathLibrary.RandomIntegerInRange` 3 10)))
        (`SkeletalMeshComponent.PlayAnimation` _mesh "/Game/Blueprints/Creatures/Wolf/Animations/ANIM_Wolf_Bite.ANIM_Wolf_Bite" false)
        (`KismetSystemLibrary.Delay` 1.0)
        (`self.StopAnimation`)
        (set `self.IsHungry?` false)
        (`self.Drain Hunger`)
        (`self.Decide Next Action` false)
        (else
          (`self.Decide Next Action` false)
          (set `self.IsHungry?` false)
          (`KismetSystemLibrary.Delay` 5.0)
          (set `self.IsHungry?` true))))))

(event `Take Damage`
  (bind _charactermovement (`self.CharacterMovement`))
  ;[1 1 1] Take Damage
  (if (not (`self.IsDead?`))
    (bind _output_get (set `self.Health` (`KismetMathLibrary.Clamp` (- (`self.Health`) (`self.Damage`)) 0 (`self.MaxHealth`))))
    (if (== _output_get 0)
      (`MovementComponent.StopMovementImmediately` _charactermovement)
      (set `self.IsDead?` true)
      (`CharacterMovementComponent.DisableMovement` (`self.CharacterMovement`))
      (`self.PlayAnimation` "/Game/Blueprints/Creatures/Wolf/Animations/ANIM_Wolf_Death.ANIM_Wolf_Death")
      ;;[1 1 1] De-spawn
      (`KismetSystemLibrary.Delay` (`KismetMathLibrary.Conv_IntToDouble` (`KismetMathLibrary.RandomIntegerInRange` 60 120)))
      (`self.K2_DestroyActor`)
      (else
        (`MovementComponent.StopMovementImmediately` _charactermovement)
        (`self.PlayAnimation` "/Game/Blueprints/Creatures/Wolf/Animations/ANIM_Wolf_GetHitFront.ANIM_Wolf_GetHitFront")
        (set `self.ShouldRun?` true)
        (`KismetSystemLibrary.Delay` 0.7)
        (`self.StopAnimation`)
        (if (not (`self.IsDead?`))
          (`self.Decide Next Action` true))))))

(event `Drain Hunger`
  ;[1 1 1] DrainHunger
  (if (not (`self.IsHungry?`))
    (bind _output_get (set `self.Hunger` (`KismetMathLibrary.Clamp` (- (`self.Hunger`) (`self.HungerDrain`)) 0 (`self.MaxHunger`))))
    (if (== _output_get 0)
      (set `self.IsHungry?` true)
      (`self.Decide Next Action` false)
      (else
        (`KismetSystemLibrary.Delay` 1.0)
        (`self.Drain Hunger`)))))

(event `Add Hunger`
  ;[1 1 1] Regain Hunger
  (if (`self.IsHungry?`)
    (bind _output_get (set `self.Hunger` (`KismetMathLibrary.Clamp` (+ (`self.Hunger`) (`self.HungerGain`)) 0 (`self.MaxHunger`))))
    (if (not (== _output_get (`self.MaxHunger`)))
      (`KismetSystemLibrary.Delay` 1.0)
      (`self.Add Hunger`))))

(event `Regen Health`
  ;[1 1 1] Regen Health
  (if (and (< (`self.Health`) (`self.MaxHealth`)) (not (`self.ShouldRun?`)))
    (bind _output_get (set `self.Health` (`KismetMathLibrary.Clamp` (+ (`self.Health`) (`self.Health Gain`)) 0 (`self.MaxHealth`))))
    (if (not (== _output_get (`self.MaxHealth`)))
      (`KismetSystemLibrary.Delay` 1.0 :!label _label_3)
      (`self.Regen Health`))
    (else
      (goto _label_3))))

(event `self.ReceiveHit`
  (params (MyComp :type "PrimitiveComponent Object Reference") (Other :type "Actor Object Reference") (OtherComp :type "PrimitiveComponent Object Reference") (bSelfMoved :type Boolean) (HitLocation :type "Vector Structure") (HitNormal :type "Vector Structure") (NormalImpulse :type "Vector Structure") (Hit :type "HitResult Structure (by ref)"))
  ;[1 1 1] Projectile hit (OVERWRITE FUNCTIONALITY)
  (bind _asnew_projectile_bp (cast `/Game/Blueprints/NewProjectileBP` Other))
  (set `self.Damage` 10)
  (`self.Take Damage`)
  (`self.K2_DestroyActor` _asnew_projectile_bp))

(fn `DeselectCreature`
  (if (`self.IsSelectedCreature?`)
    (set `self.IsSelectedCreature?` false)))

(fn `New Creature UI`
  (`self.UpdateUIText`)
  (`self.UpdateUIMeters`))

(fn `PlayAnimation`
  (params (Animation :type "AnimationAsset Object Reference") (`ShouldLoop?` :type Boolean))
  (`SkeletalMeshComponent.PlayAnimation` (`self.Mesh`) Animation `ShouldLoop?`))

(fn `SelectCreature`
  (set `self.IsSelectedCreature?` true)
  (bind _astbcplayer_controller (cast `/Game/Blueprints/TBCPlayerController` (`GameplayStatics.GetPlayerController` 0)))
  (`self.New Creature UI`)
  (`KismetSystemLibrary.PrintString` (`KismetSystemLibrary.GetDisplayName` null)))

(fn `SetCameraForwardPosToCreature`
  (set `/Game/Blueprints/PlayerCamera.ForwardPos` (+ (`SceneComponent.K2_GetComponentLocation` (`self.Mesh`)) (-360.0 0.0 100.0)) (`self.PlayerCamera`)))

(fn `SetCreatureAnimState`)

(fn `SetHoverColor`)

(fn `SetText`
  (`TextRenderComponent.K2_SetText` (`self.CreatureName`) (`KismetTextLibrary.Conv_StringToText` (`KismetStringLibrary.Concat_StrStr` (`KismetStringLibrary.Concat_StrStr` (`KismetStringLibrary.Concat_StrStr` (`KismetStringLibrary.Concat_StrStr` (`|GetEnumeratorNameAsString` (`self.CreatureType`)) " - ") (`self.CreatureFirstName`)) " ") (`self.CreatureLastName`)))))

(fn `StopAnimation`
  (bind _mesh (`self.Mesh`))
  (`SkeletalMeshComponent.SetAnimationMode` _mesh "AnimationBlueprint")
  (`SkeletalMeshComponent.SetAnimInstanceClass` _mesh null))

(fn `UpdateUIMeters`
  (bind _astbchud (cast `/Game/Blueprints/Widgets/TBCHud` (`PlayerController.GetHUD` (`GameplayStatics.GetPlayerController` 0))))
  (`/Game/Blueprints/Widgets/TBCUI.UpdateMeters` (`/Game/Blueprints/Widgets/TBCHud.UI Ref` _astbchud) (`KismetMathLibrary.Conv_IntToDouble` (`self.Health`)) (`KismetMathLibrary.Conv_IntToDouble` (`self.Hunger`)) (`KismetMathLibrary.Conv_IntToDouble` (`self.MaxHealth`)) (`KismetMathLibrary.Conv_IntToDouble` (`self.MaxHunger`)) (`KismetMathLibrary.Conv_IntToDouble` (`self.Energy`)) (`KismetMathLibrary.Conv_IntToDouble` (`self.MaxEnergy`))))

(fn `UpdateUIText`
  (bind _astbchud (cast `/Game/Blueprints/Widgets/TBCHud` (`PlayerController.GetHUD` (`GameplayStatics.GetPlayerController` 0))))
  (`/Game/Blueprints/Widgets/TBCUI.UpdateText` (`/Game/Blueprints/Widgets/TBCHud.UI Ref` _astbchud) (`KismetTextLibrary.Conv_StringToText` (`KismetStringLibrary.Concat_StrStr` (`KismetStringLibrary.Concat_StrStr` (`self.CreatureFirstName`) " ") (`self.CreatureLastName`))) (`KismetTextLibrary.Conv_StringToText` (`|GetEnumeratorNameAsString` (`self.CreatureType`))) (`KismetTextLibrary.Conv_StringToText` (`|GetEnumeratorNameAsString` (`self.CurrentActivity`))) (`KismetTextLibrary.Conv_StringToText` (`|GetEnumeratorNameAsString` (`self.CreatureJob`)))))

(fn `UserConstructionScript`)