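; Base character for wolf, crocodile and pig clan creatures in a tribe-management game, with random stats, age, hover name labels and click selection that drives the HUD.
; Creatures roam via AIMoveTo, die, and breed through a timeline-driven pregnancy limited to one baby per clan, spawning half-scale children who later fill empty clan roles.
; Job-specific council buttons add tooltip modifiers to clan resource daily rates and shift inter-clan relations.
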(event `INIT_CreatureBase`
  (bind _returnvalue (`GameplayStatics.GetPlayerController` 0))
  (set `self.CursorStatus` "NewEnumerator0")
  (set `self.CurrentActivity` "NewEnumerator0")
  (bind _astbcplayer_controller (cast `/Game/Blueprints/TBCPlayerController` _returnvalue))
  (set `self.PlayerCamera` (`/Game/Blueprints/TBCPlayerController.TBCPlayerCamera` _astbcplayer_controller))
  (set `self.TBCPlayerController` _astbcplayer_controller)
  (bind _astbchud (cast `/Game/Blueprints/Widgets/TBCHud` (`PlayerController.GetHUD` _returnvalue)))
  (bind _output_get (set `self.TBCHud` _astbchud))
  (bind _output_get_2 (set `self.TBCUI` (`/Game/Blueprints/Widgets/TBCHud.TBCUI` _output_get)))
  (set `self.OtherTribesParent` (`/Game/Blueprints/Widgets/TBCUI.TBCOtherTribesParent` _output_get_2))
  (bind _astbcgame_state (cast `/Game/Blueprints/TBCGameState` (`GameplayStatics.GetGameState`)))
  (set `self.TBCGameState` _astbcgame_state)
  (`self.SetText`)
  (`self.Random Roam`)
  (`self.SetStatsRandom`)
  (`self.SETLOGIC_ResourceBar`)
  (set `self.HittingOtherCreature` false)
  (`self.Set Age Random` (`self.IsChild`))
  (`SceneComponent.SetVisibility` (`self.CreatureName`) false false :!label _label))

(event `self.ReceiveTick`
  (params (DeltaSeconds :type "Float (single-precision)")))

(event `self.Mesh.OnEndCursorOver`
  (params (TouchedComponent :type "PrimitiveComponent Object Reference"))
  (set `self.CursorStatus` "NewEnumerator0")
  (goto _label))

(event `self.Mesh.OnClicked`
  (params (TouchedComponent :type "PrimitiveComponent Object Reference") (ButtonPressed :type "Key Structure"))
  (bind _mycreaturetype (`self.MyCreatureType`))
  (bind _tbcui (`/Game/Blueprints/Widgets/TBCHud.TBCUI` (`self.TBCHud`)))
  (set `self.CursorStatus` "NewEnumerator2")
  (`/Game/Blueprints/TBCGameState.SetSelectedCreature` (`self.TBCGameState`) self)
  (`self.UpdateCouncil`)
  (`/Game/Blueprints/Widgets/ResourceBar/TBCResourceBarsParent.SetClanVisible` (`/Game/Blueprints/Widgets/TBCUI.TBCResourceBarsParent` _tbcui) _mycreaturetype)
  (`/Game/Blueprints/Widgets/OtherTribes/TBCOtherTribesParent.SetClanVisible` (`/Game/Blueprints/Widgets/TBCUI.TBCOtherTribesParent` _tbcui) _mycreaturetype)
  (`SceneComponent.SetVisibility` (`self.CreatureName`) true false :!label _label_2))

(event `self.Mesh.OnBeginCursorOver`
  (params (TouchedComponent :type "PrimitiveComponent Object Reference"))
  (set `self.CursorStatus` "NewEnumerator1")
  (goto _label_2))

(event `self.Mesh.OnReleased`
  (params (TouchedComponent :type "PrimitiveComponent Object Reference") (ButtonReleased :type "Key Structure"))
  (set `self.CursorStatus` "NewEnumerator1")
  (goto _label_2))

(event `Decide Next Behaviour`
  (params (`SkipDelay?` :type Boolean) (Behaviour :type "/Game/Blueprints/Creatures/CreatureActivity Enum" :default "NewEnumerator0"))
  ;[1 1 1] AI Decision Tree
  (if (not `SkipDelay?`)
    (`KismetSystemLibrary.Delay` (`KismetMathLibrary.Conv_IntToDouble` (`KismetMathLibrary.RandomIntegerInRange` 1 5))))
  (`self.Random Roam`))

(event `Random Roam`
  ;[1 1 1] Random Roam
  (set `self.CurrentActivity` "NewEnumerator1")
  (set `CharacterMovementComponent.MaxWalkSpeed` 150.0 (`self.CharacterMovement`))
  (`|AIMoveTo` self (`NavigationSystemV1.K2_GetRandomReachablePointInRadius` (`self.K2_GetActorLocation`) 1500.0 null null) null 5.0 true
    (:`OnSuccess`
      (`self.Decide Next Behaviour` self false "NewEnumerator0"))))

(event `Die`
  ;[1 1 1] Creature Death
  (`/Game/Blueprints/Widgets/TBCUI.HOLISTIC_TriggerEvent` (`/Game/Blueprints/Widgets/TBCHud.TBCUI` (`self.TBCHud`)) (`KismetTextLibrary.Conv_StringToText` (`KismetStringLibrary.Concat_StrStr` "Oh no! " (`|GetEnumeratorNameAsString` (`self.CreatureJob`)) " " (`self.CreatureFirstName`) " " (`self.CreatureLastName`) " has died at age " (`KismetStringLibrary.Conv_IntToString` (`self.Age`)) "!")) "NewEnumerator1" null null)
  (set `self.CurrentActivity` "NewEnumerator7")
  (`/Game/Blueprints/TBCGameState.RemoveDeadCreature` (`self.TBCGameState`) self))

(event `BecomePregnant`
  (params (CreatureType :type "/Game/Blueprints/Creatures/CreatureTypes Enum" :default "NewEnumerator0"))
  (bind _tbcgamestate (`self.TBCGameState`))
  (bind _tbcui (`self.TBCUI`))
  (bind _wolfclan (`/Game/Blueprints/TBCGameState.WolfClan` _tbcgamestate))
  (bind _crocclan (`/Game/Blueprints/TBCGameState.CrocClan` _tbcgamestate))
  (bind _pigclan (`/Game/Blueprints/TBCGameState.PigClan` _tbcgamestate))
  ;[1 1 1] Check if there is already a child
  (switch `/Game/Blueprints/Creatures/CreatureTypes` CreatureType
    (:`NewEnumerator0`
      (bind _haspregnantanimal (`/Game/Blueprints/TBCClan.HasPregnantClanMember` _wolfclan))
      (if (not (or (`/Game/Blueprints/TBCClan.HasBaby` _wolfclan) _haspregnantanimal))
        ;[1 1 1] Check if creature is already pregnant
        (if (not (`self.IsPregnant`)) :!label _label_3
          (set `self.IsPregnant` true)
          (`/Game/Blueprints/Widgets/TBCUI.EnablePregnancyUI` _tbcui)
          (`/Game/Blueprints/Widgets/TBCUI.SETVISUAL_PregnantText` _tbcui (`self.IsPregnant`))
          (bind (_direction _pregnancypercent) (`Timeline|PregnancyTimeline` :`NewTime` 10.0 :!via `PlayFromStart`)
            (:`Update`
              (`/Game/Blueprints/Widgets/TBCUI.SETVISUALS_PregnancyBar` _tbcui _pregnancypercent 1.0))
            (:`Finished`
              (`self.BirthNewCreature`))))))
    (:`NewEnumerator1`
      (bind _haspregnantanimal_2 (`/Game/Blueprints/TBCClan.HasPregnantClanMember` _crocclan))
      (if (not (or (`/Game/Blueprints/TBCClan.HasBaby` _crocclan) _haspregnantanimal_2))
        (goto _label_3)))
    (:`NewEnumerator10`
      (bind _haspregnantanimal_3 (`/Game/Blueprints/TBCClan.HasPregnantClanMember` _pigclan))
      (if (not (or (`/Game/Blueprints/TBCClan.HasBaby` _pigclan) _haspregnantanimal_3))
        (goto _label_3)))))

(event `BirthNewCreature`
  (bind _tbcui (`self.TBCUI`))
  (bind _tbcui_2 (`self.TBCUI`))
  (bind _output_get (set `self.CurrentActivity` "NewEnumerator8"))
  (`/Game/Blueprints/Widgets/TBCUI.SETVISUAL_ActionText` _tbcui _output_get)
  (`KismetSystemLibrary.Delay` (`KismetMathLibrary.RandomFloatInRange` 1.0 2.0))
  (`/Game/Blueprints/Widgets/TBCUI.DisablePregnancyUI` _tbcui)
  (`self.SpawnChild`)
  (bind _output_get_2 (set `self.CurrentActivity` "NewEnumerator1"))
  (`/Game/Blueprints/Widgets/TBCUI.SETVISUAL_ActionText` _tbcui_2 _output_get_2)
  (bind _output_get_3 (set `self.IsPregnant` false))
  (`/Game/Blueprints/Widgets/TBCUI.SETVISUAL_PregnantText` _tbcui_2 _output_get_3)
  (`KismetSystemLibrary.PrintString` "Creature birth ended"))

(event `SpawnChild`
  (bind _returnvalue (`self.GetTransform`))
  (bind _mycreaturetype (`self.MyCreatureType`))
  (bind _tbcgamestate (`self.TBCGameState`))
  (bind _tbchud (`self.TBCHud`))
  ;[1 1 1] Spawn Child from this creature
  (switch `/Game/Blueprints/Creatures/CreatureTypes` _mycreaturetype
    (:`NewEnumerator0`
      (bind _returnvalue_2 (`|SpawnActorFromClass` "/Game/Blueprints/Creatures/Wolf/Wolf.Wolf_C" _returnvalue "AlwaysSpawn" "OverrideRootScale" null (0.0 0.0 0.0) null))
      (set `/Game/Blueprints/Creatures/CreatureBase.MyCreatureType` _mycreaturetype _returnvalue_2)
      (`self.SetActorScale3D` _returnvalue_2 (0.5 0.5 0.5))
      (bind _output_get (set `/Game/Blueprints/Creatures/CreatureBase.IsChild` true _returnvalue_2))
      (`self.Set Age Random` _returnvalue_2 _output_get)
      (`self.INIT_CreatureBase` _returnvalue_2)
      (`/Game/Blueprints/TBCGameState.SetSelectedCreature` _tbcgamestate _returnvalue_2)
      (`self.SetCreatureJob` _returnvalue_2 "NewEnumerator6")
      (`/Game/Blueprints/TBCGameState.Add New Creature` _tbcgamestate "NewEnumerator0" _returnvalue_2)
      (`/Game/Blueprints/Widgets/TBCUI.HOLISTIC_TriggerEvent` (`/Game/Blueprints/Widgets/TBCHud.TBCUI` _tbchud) "A baby wolf has been born!" "NewEnumerator0" _returnvalue_2 self)
      (`self.UpdateStatVisuals` _returnvalue_2)
      (`self.SETVISUALS_CreatureDetails` _returnvalue_2)
      (`self.SETVISUALS_CreatureDetails` _returnvalue_2))
    (:`NewEnumerator1`
      (bind _returnvalue_3 (`|SpawnActorFromClass` "/Game/Blueprints/Creatures/Crocodile/Crocodile.Crocodile_C" _returnvalue "AlwaysSpawn" "OverrideRootScale" null (0.0 0.0 0.0) null))
      (set `/Game/Blueprints/Creatures/CreatureBase.MyCreatureType` _mycreaturetype _returnvalue_3)
      (`self.SetActorScale3D` _returnvalue_3 (0.5 0.5 0.5))
      (bind _output_get_2 (set `/Game/Blueprints/Creatures/CreatureBase.IsChild` true _returnvalue_3))
      (`self.Set Age Random` _returnvalue_3 _output_get_2)
      (`self.INIT_CreatureBase` _returnvalue_3)
      (`/Game/Blueprints/TBCGameState.SetSelectedCreature` _tbcgamestate _returnvalue_3)
      (`self.SetCreatureJob` _returnvalue_3 "NewEnumerator6")
      (`/Game/Blueprints/TBCGameState.Add New Creature` _tbcgamestate "NewEnumerator1" _returnvalue_3)
      (`/Game/Blueprints/Widgets/TBCUI.HOLISTIC_TriggerEvent` (`/Game/Blueprints/Widgets/TBCHud.TBCUI` _tbchud) "A baby croc has been born!" "NewEnumerator0" _returnvalue_3 self)
      (`self.UpdateStatVisuals` _returnvalue_3)
      (`self.SETVISUALS_CreatureDetails` _returnvalue_3))
    (:`NewEnumerator10`
      (bind _returnvalue_4 (`|SpawnActorFromClass` "/Game/Blueprints/Creatures/Pig/Pig.Pig_C" _returnvalue "AlwaysSpawn" "OverrideRootScale" null (0.0 0.0 0.0) null))
      (set `/Game/Blueprints/Creatures/CreatureBase.MyCreatureType` _mycreaturetype _returnvalue_4)
      (`self.SetActorScale3D` _returnvalue_4 (0.5 0.5 0.5))
      (bind _output_get_3 (set `/Game/Blueprints/Creatures/CreatureBase.IsChild` true _returnvalue_4))
      (`self.Set Age Random` _returnvalue_4 _output_get_3)
      (`self.INIT_CreatureBase` _returnvalue_4)
      (`/Game/Blueprints/TBCGameState.SetSelectedCreature` _tbcgamestate _returnvalue_4)
      (`self.SetCreatureJob` _returnvalue_4 "NewEnumerator6")
      (`/Game/Blueprints/TBCGameState.Add New Creature` _tbcgamestate "NewEnumerator10" _returnvalue_4)
      (`/Game/Blueprints/Widgets/TBCUI.HOLISTIC_TriggerEvent` (`/Game/Blueprints/Widgets/TBCHud.TBCUI` _tbchud) "A baby pig has been born!" "NewEnumerator0" _returnvalue_4 self)
      (`self.UpdateStatVisuals` _returnvalue_4)
      (`self.SETVISUALS_CreatureDetails` _returnvalue_4))))

(event `AgeWolfChildUp`
  (bind _wolfclan (`/Game/Blueprints/TBCGameState.WolfClan` (`self.TBCGameState`)))
  ;[1 1 1] Child Age Up
  (if (`/Game/Blueprints/TBCClan.HasBaby` _wolfclan)
    (bind (_emptyrole _hasemptyrole) (`/Game/Blueprints/TBCClan.ClanHasEmptyRole` _wolfclan))
    (if _hasemptyrole
      (`self.SetActorScale3D` (1.0 1.0 1.0))
      (`self.WolfFindOpenWorkSpot`))))

(event `WolfFindOpenWorkSpot`
  ;[1 1 1] Child Age Up
  (`self.SetCreatureJob` (stale `AgeWolfChildUp` _emptyrole))
  (set `/Game/Blueprints/TBCClan.HasBaby` false (`/Game/Blueprints/TBCGameState.WolfClan` (`self.TBCGameState`)))
  (`self.SETVISUALS_CreatureDetails`)
  (`self.UpdateCouncil`)
  (`self.UpdateStatVisuals`))

(event `AgeCrocChildUp`
  (bind _crocclan (`/Game/Blueprints/TBCGameState.CrocClan` (`self.TBCGameState`)))
  ;[1 1 1] Child Age Up
  (if (`/Game/Blueprints/TBCClan.HasBaby` _crocclan)
    (bind (_emptyrole _hasemptyrole) (`/Game/Blueprints/TBCClan.ClanHasEmptyRole` _crocclan))
    (if _hasemptyrole
      (`self.SetActorScale3D` (1.0 1.0 1.0))
      (`self.CrocFindOpenWorkSpot`))))

(event `CrocFindOpenWorkSpot`
  ;[1 1 1] Child Age Up
  (`self.SetCreatureJob` (stale `AgeCrocChildUp` _emptyrole))
  (set `/Game/Blueprints/TBCClan.HasBaby` false (`/Game/Blueprints/TBCGameState.CrocClan` (`self.TBCGameState`)))
  (`self.SETVISUALS_CreatureDetails`)
  (`self.UpdateCouncil`)
  (`self.UpdateStatVisuals`))

(event `AgePigChildUp`
  (bind _pigclan (`/Game/Blueprints/TBCGameState.PigClan` (`self.TBCGameState`)))
  ;[1 1 1] Child Age Up
  (if (`/Game/Blueprints/TBCClan.HasBaby` _pigclan)
    (bind (_emptyrole _hasemptyrole) (`/Game/Blueprints/TBCClan.ClanHasEmptyRole` _pigclan))
    (if _hasemptyrole
      (`self.SetActorScale3D` (1.0 1.0 1.0))
      (`self.PigFindOpenWorkSpot`))))

(event `PigFindOpenWorkSpot`
  ;[1 1 1] Child Age Up
  (`self.SetCreatureJob` (stale `AgePigChildUp` _emptyrole))
  (set `/Game/Blueprints/TBCClan.HasBaby` false (`/Game/Blueprints/TBCGameState.PigClan` (`self.TBCGameState`)))
  (`self.SETVISUALS_CreatureDetails`)
  (`self.UpdateCouncil`)
  (`self.UpdateStatVisuals`))

(fn `Calculate Tribe Relation Daily Rate Other Clans`
  (params (MainClan :type "/Game/Blueprints/Creatures/CreatureTypes Enum" :default "NewEnumerator0") (`Daily Rate Add Amount` :type "Float (double-precision)"))
  (bind _othertribesparent (`self.OtherTribesParent`))
  (switch `/Game/Blueprints/Creatures/CreatureTypes` MainClan
    (:`NewEnumerator0`
      (`/Game/Blueprints/Widgets/OtherTribes/TBCOtherTribesParent.Add To Wolf Pig Relation Daily Rate` _othertribesparent `Daily Rate Add Amount`)
      (`/Game/Blueprints/Widgets/OtherTribes/TBCOtherTribesParent.Add To Croc Wolf Relation Daily Rate` _othertribesparent `Daily Rate Add Amount`))
    (:`NewEnumerator1`
      (`/Game/Blueprints/Widgets/OtherTribes/TBCOtherTribesParent.Add To Pig Croc Relation Daily Rate` _othertribesparent `Daily Rate Add Amount`)
      (`/Game/Blueprints/Widgets/OtherTribes/TBCOtherTribesParent.Add To Croc Wolf Relation Daily Rate` _othertribesparent `Daily Rate Add Amount`))
    (:`NewEnumerator10`
      (`/Game/Blueprints/Widgets/OtherTribes/TBCOtherTribesParent.Add To Wolf Pig Relation Daily Rate` _othertribesparent `Daily Rate Add Amount`)
      (`/Game/Blueprints/Widgets/OtherTribes/TBCOtherTribesParent.Add To Pig Croc Relation Daily Rate` _othertribesparent `Daily Rate Add Amount`))))

(fn `Calculate Tribe Relation Daily Rate Two Clans`
  (params (CreatureType1 :type "/Game/Blueprints/Creatures/CreatureTypes Enum" :default "NewEnumerator0") (CreatureType2 :type "/Game/Blueprints/Creatures/CreatureTypes Enum" :default "NewEnumerator0") (Amount :type "Float (double-precision)"))
  (bind _othertribesparent (`self.OtherTribesParent`))
  ;[1 1 1] Update Specific Tribe to Tribe Daily Rate relation
  (switch `/Game/Blueprints/Creatures/CreatureTypes` CreatureType1
    (:`NewEnumerator0`
      (switch `/Game/Blueprints/Creatures/CreatureTypes` CreatureType2
        (:`NewEnumerator1`
          (`/Game/Blueprints/Widgets/OtherTribes/TBCOtherTribesParent.Add To Croc Wolf Relation Daily Rate` _othertribesparent Amount))
        (:`NewEnumerator10`
          (`/Game/Blueprints/Widgets/OtherTribes/TBCOtherTribesParent.Add To Wolf Pig Relation Daily Rate` _othertribesparent Amount))))
    (:`NewEnumerator1`
      (switch `/Game/Blueprints/Creatures/CreatureTypes` CreatureType2
        (:`NewEnumerator0`
          (`/Game/Blueprints/Widgets/OtherTribes/TBCOtherTribesParent.Add To Croc Wolf Relation Daily Rate` _othertribesparent Amount))
        (:`NewEnumerator10`
          (`/Game/Blueprints/Widgets/OtherTribes/TBCOtherTribesParent.Add To Pig Croc Relation Daily Rate` _othertribesparent Amount))))
    (:`NewEnumerator10`
      (switch `/Game/Blueprints/Creatures/CreatureTypes` CreatureType2
        (:`NewEnumerator0`
          (`/Game/Blueprints/Widgets/OtherTribes/TBCOtherTribesParent.Add To Wolf Pig Relation Daily Rate` _othertribesparent Amount))
        (:`NewEnumerator1`
          (`/Game/Blueprints/Widgets/OtherTribes/TBCOtherTribesParent.Add To Pig Croc Relation Daily Rate` _othertribesparent Amount))))))

(fn `CalculateResourceDailyRate`
  (params (ResourceType :type "/Game/Blueprints/ResourceTypes Enum" :default "NewEnumerator0") (ModifierHours :type "Float (double-precision)") (Description :type String) (ModifierAmount :type "Float (double-precision)") (Identification :type "/Game/Blueprints/Widgets/ResourceBar/ResourceModifierIdentification Enum" :default "NewEnumerator0") (ModifierType :type "/Game/Blueprints/Widgets/ResourceBar/ResourceModifiersType Enum" :default "NewEnumerator0") (AssociatedCreature :type "/Game/Blueprints/Creatures/CreatureBase Object Reference"))
  (returns (NewDailyRate :type "Float (double-precision)"))
  (locals (DailyRateCalculationVar :type "Float (double-precision)"))
  (bind _resourcebar (`/Game/Blueprints/TBCClan.ResourceBar` (`self.MyClan`)))
  (bind _tooltip (`/Game/Blueprints/Widgets/ResourceBar/TBCResourceBox.Tooltip` (`/Game/Blueprints/Widgets/ResourceBar/TBCResourceBar.DramaBox` _resourcebar)))
  (bind _tooltip_2 (`/Game/Blueprints/Widgets/ResourceBar/TBCResourceBox.Tooltip` (`/Game/Blueprints/Widgets/ResourceBar/TBCResourceBar.PietyBox` _resourcebar)))
  (bind _tooltip_3 (`/Game/Blueprints/Widgets/ResourceBar/TBCResourceBox.Tooltip` (`/Game/Blueprints/Widgets/ResourceBar/TBCResourceBar.PopulationBox` _resourcebar)))
  (bind _tooltip_4 (`/Game/Blueprints/Widgets/ResourceBar/TBCResourceBox.Tooltip` (`/Game/Blueprints/Widgets/ResourceBar/TBCResourceBar.FoodBox` _resourcebar)))
  (bind _tooltip_5 (`/Game/Blueprints/Widgets/ResourceBar/TBCResourceBox.Tooltip` (`/Game/Blueprints/Widgets/ResourceBar/TBCResourceBar.InfluenceBox` _resourcebar)))
  (set `local.DailyRateCalculationVar` 0.0)
  (switch `/Game/Blueprints/ResourceTypes` ResourceType
    (:`NewEnumerator0`
      (`/Game/Blueprints/Widgets/Tooltips/TBCResourceTooltip.CreateNewModifier` _tooltip_3 ModifierType Description ModifierAmount ResourceType ModifierHours Identification)
      (for _array_element (`/Game/Blueprints/Widgets/Tooltips/TBCResourceTooltip.Modifiers` _tooltip_3)
        (set `local.DailyRateCalculationVar` (+ (`/Game/Blueprints/Widgets/Tooltips/TBCResourceModifier.ModifierNumber` _array_element) (`local.DailyRateCalculationVar`)))
        (return (`local.DailyRateCalculationVar`))))
    (:`NewEnumerator1`
      (`/Game/Blueprints/Widgets/Tooltips/TBCResourceTooltip.CreateNewModifier` _tooltip_4 ModifierType Description ModifierAmount ResourceType ModifierHours Identification)
      (for _array_element_2 (`/Game/Blueprints/Widgets/Tooltips/TBCResourceTooltip.Modifiers` _tooltip_4)
        (set `local.DailyRateCalculationVar` (+ (`/Game/Blueprints/Widgets/Tooltips/TBCResourceModifier.ModifierNumber` _array_element_2) (`local.DailyRateCalculationVar`)))
        (return (`local.DailyRateCalculationVar`))))
    (:`NewEnumerator2`
      (`/Game/Blueprints/Widgets/Tooltips/TBCResourceTooltip.CreateNewModifier` _tooltip_5 ModifierType Description ModifierAmount ResourceType ModifierHours Identification)
      (for _array_element_3 (`/Game/Blueprints/Widgets/Tooltips/TBCResourceTooltip.Modifiers` _tooltip_5)
        (set `local.DailyRateCalculationVar` (+ (`/Game/Blueprints/Widgets/Tooltips/TBCResourceModifier.ModifierNumber` _array_element_3) (`local.DailyRateCalculationVar`)))
        (return (`local.DailyRateCalculationVar`))))
    (:`NewEnumerator3`
      (`/Game/Blueprints/Widgets/Tooltips/TBCResourceTooltip.CreateNewModifier` _tooltip_2 ModifierType Description ModifierAmount ResourceType ModifierHours Identification)
      (for _array_element_4 (`/Game/Blueprints/Widgets/Tooltips/TBCResourceTooltip.Modifiers` _tooltip_2)
        (set `local.DailyRateCalculationVar` (+ (`/Game/Blueprints/Widgets/Tooltips/TBCResourceModifier.ModifierNumber` _array_element_4) (`local.DailyRateCalculationVar`)))
        (return (`local.DailyRateCalculationVar`))))
    (:`NewEnumerator4`
      (`/Game/Blueprints/Widgets/Tooltips/TBCResourceTooltip.CreateNewModifier` _tooltip ModifierType Description ModifierAmount ResourceType ModifierHours Identification)
      (for _array_element_5 (`/Game/Blueprints/Widgets/Tooltips/TBCResourceTooltip.Modifiers` _tooltip)
        (set `local.DailyRateCalculationVar` (+ (`/Game/Blueprints/Widgets/Tooltips/TBCResourceModifier.ModifierNumber` _array_element_5) (`local.DailyRateCalculationVar`)))
        (return (`local.DailyRateCalculationVar`))))))

(fn `DeselectCreature`
  (if (`self.IsSelectedCreature?`)
    (set `self.IsSelectedCreature?` false)))

(fn `First Council Role Button Pressed`
  (switch `/Game/Blueprints/Creatures/CreatureJobEnum` (`self.CreatureJob`)
    (:`NewEnumerator0`
      (set `self.ArdentActions` "NewEnumerator0")
      (bind _newdailyrate (`self.CalculateResourceDailyRate` "NewEnumerator2" -1.0 "ardent talks to other clans" 5.0 "NewEnumerator2" "NewEnumerator0" self))
      (`/Game/Blueprints/TBCClan.SENDINFO_Clan Resource Daily Rate` (`self.MyClan`) _newdailyrate "NewEnumerator2")
      (`self.Calculate Tribe Relation Daily Rate Other Clans` self (`self.MyCreatureType`) 0.05))
    (:`NewEnumerator1`
      (set `self.BrewdActions` "NewEnumerator0")
      (bind _newdailyrate_2 (`self.CalculateResourceDailyRate` "NewEnumerator1" -1.0 "prepare meals selected by brewd in council" 5.0 "NewEnumerator0" "NewEnumerator0" self))
      (`/Game/Blueprints/TBCClan.SENDINFO_Clan Resource Daily Rate` (`self.MyClan`) _newdailyrate_2 "NewEnumerator1"))
    (:`NewEnumerator2`
      (set `self.ShamanActions` "NewEnumerator0"))
    (:`NewEnumerator4`
      (set `self.SoothSayerActions` "NewEnumerator0"))
    (:`NewEnumerator3`
      (set `self.MidwifeActions` "NewEnumerator0"))
    (:`NewEnumerator6`
      (set `self.ChildActions` "NewEnumerator0"))))

(fn `GetCreatureName`
  (returns (Name :type Name))
  (return (`KismetStringLibrary.Conv_StringToName` (`KismetStringLibrary.Concat_StrStr` (`KismetStringLibrary.Concat_StrStr` (`self.CreatureFirstName`) " ") (`self.CreatureLastName`)))))

(fn `New Creature UI`
  (`self.SETVISUALS_CreatureDetails`)
  (`self.UpdateUIMeters`)
  (`self.UpdateStatVisuals`))

(fn `PlayAnimation`
  (params (Animation :type "AnimationAsset Object Reference") (`ShouldLoop?` :type Boolean))
  (`SkeletalMeshComponent.PlayAnimation` (`self.Mesh`) Animation `ShouldLoop?`))

(fn `Second Council Role Button Pressed`
  (switch `/Game/Blueprints/Creatures/CreatureJobEnum` (`self.CreatureJob`)
    (:`NewEnumerator0`
      (set `self.ArdentActions` "NewEnumerator1")
      (bind _newdailyrate (`self.CalculateResourceDailyRate` "NewEnumerator2" -1.0 "ardent intimidates other clans" 5.0 "NewEnumerator2" "NewEnumerator0" self))
      (`/Game/Blueprints/TBCClan.SENDINFO_Clan Resource Daily Rate` (`self.MyClan`) _newdailyrate "NewEnumerator2")
      (`self.Calculate Tribe Relation Daily Rate Other Clans` self (`self.MyCreatureType`) -0.03))
    (:`NewEnumerator1`
      (set `self.BrewdActions` "NewEnumerator1")
      (bind _newdailyrate_2 (`self.CalculateResourceDailyRate` "NewEnumerator1" -1.0 "Forage selected by Brewd" 2.0 "NewEnumerator0" "NewEnumerator0" self))
      (`/Game/Blueprints/TBCClan.SENDINFO_Clan Resource Daily Rate` (`self.MyClan`) _newdailyrate_2 "NewEnumerator1"))
    (:`NewEnumerator2`
      (set `self.ShamanActions` "NewEnumerator1"))
    (:`NewEnumerator4`
      (set `self.SoothSayerActions` "NewEnumerator1"))
    (:`NewEnumerator3`
      (set `self.MidwifeActions` "NewEnumerator1"))
    (:`NewEnumerator6`
      (set `self.ChildActions` "NewEnumerator1"))))

(fn `SelectCreature`
  (bind _tbcui (`/Game/Blueprints/TBCPlayerController.TBCUI` (`self.TBCPlayerController`)))
  (set `self.IsSelectedCreature?` true)
  (`/Game/Blueprints/PlayerCamera.SetSelectedCreature` (`/Game/Blueprints/TBCPlayerController.TBCPlayerCamera` (`self.TBCPlayerController`)) self)
  (`self.New Creature UI`)
  (if (`self.IsPregnant`)
    (`/Game/Blueprints/Widgets/TBCUI.EnablePregnancyUI` _tbcui)
    (else
      (`/Game/Blueprints/Widgets/TBCUI.DisablePregnancyUI` _tbcui))))

(fn `Set Age Random`
  (params (IsChild :type Boolean))
  (if IsChild
    (set `self.Age` 0)
    (else
      (set `self.Age` (`KismetMathLibrary.RandomIntegerInRange` 18 60)))))

(fn `SetAge`)

(fn `SetCameraForwardPosToCreature`
  (set `/Game/Blueprints/PlayerCamera.ForwardPos` (+ (`SceneComponent.K2_GetComponentLocation` (`self.Mesh`)) (-360.0 0.0 100.0)) (`self.PlayerCamera`)))

(fn `SetCreatureAnimState`)

(fn `SetCreatureJob`
  (params (Job :type "/Game/Blueprints/Creatures/CreatureJobEnum Enum" :default "NewEnumerator0"))
  (set `self.CreatureJob` Job))

(fn `SetHoverColor`)

(fn `SETLOGIC_ResourceBar`
  (bind _mycreaturetype (`self.MyCreatureType`))
  (bind _tbcresourcebarsparent (`/Game/Blueprints/Widgets/TBCUI.TBCResourceBarsParent` (`self.TBCUI`)))
  (switch `/Game/Blueprints/Creatures/CreatureTypes` _mycreaturetype
    (:`NewEnumerator0`
      (bind _newparam (`/Game/Blueprints/Widgets/ResourceBar/TBCResourceBarsParent.GetResourceBar` _tbcresourcebarsparent _mycreaturetype))
      (set `self.MyResourceBar` _newparam))
    (:`NewEnumerator1`
      (bind _newparam_2 (`/Game/Blueprints/Widgets/ResourceBar/TBCResourceBarsParent.GetResourceBar` _tbcresourcebarsparent _mycreaturetype))
      (set `self.MyResourceBar` _newparam_2))
    (:`NewEnumerator10`
      (bind _newparam_3 (`/Game/Blueprints/Widgets/ResourceBar/TBCResourceBarsParent.GetResourceBar` _tbcresourcebarsparent _mycreaturetype))
      (set `self.MyResourceBar` _newparam_3))))

(fn `SetStatsRandom`
  (bind _statarray (`self.StatArray`))
  (bind _output_get (set `self.Gumption` (`KismetMathLibrary.RandomIntegerInRange` 0 20)))
  (bind _output_get_2 (set `self.Taste` (`KismetMathLibrary.RandomIntegerInRange` 0 20)))
  (bind _output_get_3 (set `self.Piety` (`KismetMathLibrary.RandomIntegerInRange` 0 20)))
  (bind _output_get_4 (set `self.Memory` (`KismetMathLibrary.RandomIntegerInRange` 0 20)))
  (bind _output_get_5 (set `self.Instinct` (`KismetMathLibrary.RandomIntegerInRange` 0 20)))
  (`KismetArrayLibrary.Array_Add` _statarray _output_get)
  (`KismetArrayLibrary.Array_Add` _statarray _output_get_2)
  (`KismetArrayLibrary.Array_Add` _statarray _output_get_3)
  (`KismetArrayLibrary.Array_Add` _statarray _output_get_4)
  (`KismetArrayLibrary.Array_Add` _statarray _output_get_5))

(fn `SetText`
  (`TextRenderComponent.K2_SetText` (`self.CreatureName`) (`KismetTextLibrary.Conv_StringToText` (`KismetStringLibrary.Concat_StrStr` (`KismetStringLibrary.Concat_StrStr` (`KismetStringLibrary.Concat_StrStr` (`KismetStringLibrary.Concat_StrStr` (`|GetEnumeratorNameAsString` (`self.MyCreatureType`)) " - ") (`self.CreatureFirstName`)) " ") (`self.CreatureLastName`)))))

(fn `SETVISUALS_CreatureDetails`
  (bind _astbchud (cast `/Game/Blueprints/Widgets/TBCHud` (`PlayerController.GetHUD` (`GameplayStatics.GetPlayerController` 0))))
  (bind _tbcui (`/Game/Blueprints/Widgets/TBCHud.TBCUI` _astbchud))
  (`/Game/Blueprints/Widgets/TBCUI.SETVISUAL Information Text` _tbcui (`KismetTextLibrary.Conv_NameToText` (`self.GetCreatureName`)) (`KismetTextLibrary.Conv_StringToText` (`|GetEnumeratorNameAsString` (`self.MyCreatureType`))) (`KismetTextLibrary.Conv_StringToText` (`|GetEnumeratorNameAsString` (`self.CurrentActivity`))) (`KismetTextLibrary.Conv_StringToText` (`|GetEnumeratorNameAsString` (`self.CreatureJob`))))
  (`/Game/Blueprints/Widgets/TBCUI.SETVISUAL_PregnantText` _tbcui (`self.IsPregnant`))
  (if (`self.IsChild`)
    (set `self.IsChild` true)
    (else
      (set `self.IsChild` false)))
  (`/Game/Blueprints/Widgets/TBCUI.SENDINFO Age Text` _tbcui (`self.Age`) (`self.IsChild`)))

(fn `StopAnimation`
  (bind _mesh (`self.Mesh`))
  (`SkeletalMeshComponent.SetAnimationMode` _mesh "AnimationBlueprint")
  (`SkeletalMeshComponent.SetAnimInstanceClass` _mesh null))

(fn `Third Council Button Pressed`
  (switch `/Game/Blueprints/Creatures/CreatureJobEnum` (`self.CreatureJob`)
    (:`NewEnumerator0`
      (set `self.ArdentActions` "NewEnumerator2"))
    (:`NewEnumerator1`
      (set `self.BrewdActions` "NewEnumerator2")
      (bind _newdailyrate (`self.CalculateResourceDailyRate` "NewEnumerator1" -1.0 "DevelopRecipes called from Brewd council action" 3.0 "NewEnumerator0" "NewEnumerator0" self))
      (`/Game/Blueprints/TBCClan.SENDINFO_Clan Resource Daily Rate` (`self.MyClan`) _newdailyrate "NewEnumerator1"))
    (:`NewEnumerator2`
      (set `self.ShamanActions` "NewEnumerator2"))
    (:`NewEnumerator4`
      (set `self.SoothSayerActions` "NewEnumerator2"))
    (:`NewEnumerator3`
      (set `self.MidwifeActions` "NewEnumerator2"))
    (:`NewEnumerator6`
      (set `self.ChildActions` "NewEnumerator2"))))

(fn `UpdateCouncil`
  (bind _tbcgamestate (`self.TBCGameState`))
  (bind _tbcui (`/Game/Blueprints/Widgets/TBCHud.TBCUI` (`self.TBCHud`)))
  (cast `/Game/Blueprints/Creatures/Wolf/Wolf` self
    (:`then`
      (`/Game/Blueprints/Widgets/TBCUI.Update Council Frames` _tbcui (`/Game/Blueprints/TBCClan.MyCreatures` (`/Game/Blueprints/TBCGameState.WolfClan` _tbcgamestate))))
    (:`CastFailed`
      (cast `/Game/Blueprints/Creatures/Pig/Pig` self
        (:`then`
          (`/Game/Blueprints/Widgets/TBCUI.Update Council Frames` _tbcui (`/Game/Blueprints/TBCClan.MyCreatures` (`/Game/Blueprints/TBCGameState.PigClan` _tbcgamestate))))
        (:`CastFailed`
          (cast `/Game/Blueprints/Creatures/Crocodile/Crocodile` self)
          (`/Game/Blueprints/Widgets/TBCUI.Update Council Frames` _tbcui (`/Game/Blueprints/TBCClan.MyCreatures` (`/Game/Blueprints/TBCGameState.CrocClan` _tbcgamestate))))))))

(fn `UpdateStatVisuals`
  (bind _astbchud (cast `/Game/Blueprints/Widgets/TBCHud` (`PlayerController.GetHUD` (`GameplayStatics.GetPlayerController` 0))))
  (`/Game/Blueprints/Widgets/TBCUI.SENDINFO_Stats` (`/Game/Blueprints/Widgets/TBCHud.TBCUI` _astbchud) self))

(fn `UpdateUIMeters`
  (bind _astbchud (cast `/Game/Blueprints/Widgets/TBCHud` (`PlayerController.GetHUD` (`GameplayStatics.GetPlayerController` 0))))
  (`/Game/Blueprints/Widgets/TBCUI.SETVISUAL_Needs` (`/Game/Blueprints/Widgets/TBCHud.TBCUI` _astbchud) (`KismetMathLibrary.Conv_IntToDouble` 0) (`KismetMathLibrary.Conv_IntToDouble` 0) (`KismetMathLibrary.Conv_IntToDouble` 0) (`KismetMathLibrary.Conv_IntToDouble` 0) (`KismetMathLibrary.Conv_IntToDouble` 0) (`KismetMathLibrary.Conv_IntToDouble` 0)))

(fn `UserConstructionScript`)