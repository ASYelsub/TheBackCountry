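; Wolf creature Blueprint that picks its coat materials and sets its creature type when play begins.
; After the parent BeginPlay, SetUpWolfMaterials switches on MyColor (Fur, Dark or Arctic) to assign mesh materials, then CreatureType is set.
; Fur fills two material slots, while Dark and Arctic each write both materials to a single slot, so only the second one remains.
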(event `self.ReceiveBeginPlay`
  (`parent.ReceiveBeginPlay`)
  (`self.SetUpWolfMaterials`)
  (set `self.CreatureType` "NewEnumerator0"))

(fn `SetUpWolfMaterials`
  (bind _mesh (`self.Mesh`))
  (bind _mesh_2 (`self.Mesh`))
  (bind _mesh_3 (`self.Mesh`))
  (switch `/Game/Blueprints/Creatures/WolfColors` (`self.MyColor`)
    (:`NewEnumerator0`
      (`PrimitiveComponent.SetMaterial` _mesh_2 0 "/Game/PermanentlyFreeAnimals/AnimalVarietyPack/Wolf/Materials/M_Wolf.M_Wolf")
      (`PrimitiveComponent.SetMaterial` _mesh_2 1 "/Game/PermanentlyFreeAnimals/AnimalVarietyPack/Wolf/Materials/M_WolfFur.M_WolfFur"))
    (:`NewEnumerator1`
      (`PrimitiveComponent.SetMaterial` _mesh_3 2 "/Game/PermanentlyFreeAnimals/AnimalVarietyPack/Wolf/Materials/M_WolfDark.M_WolfDark")
      (`PrimitiveComponent.SetMaterial` _mesh_3 2 "/Game/PermanentlyFreeAnimals/AnimalVarietyPack/Wolf/Materials/M_WolfFurDark.M_WolfFurDark"))
    (:`NewEnumerator2`
      (`PrimitiveComponent.SetMaterial` _mesh 1 "/Game/PermanentlyFreeAnimals/AnimalVarietyPack/Wolf/Materials/M_WolfArctic.M_WolfArctic")
      (`PrimitiveComponent.SetMaterial` _mesh 1 "/Game/PermanentlyFreeAnimals/AnimalVarietyPack/Wolf/Materials/M_WolfFurArctic.M_WolfFurArctic"))))

(fn `UserConstructionScript`
  (`parent.UserConstructionScript`))