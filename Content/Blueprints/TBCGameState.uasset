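; Game state that tracks the Wolf, Pig and Crocodile creature groups and which creature is selected.
; On BeginPlay it gathers each group, then after a short delay selects the first Wolf and assigns jobs from array indices.
; Next and previous functions cycle with wraparound within the current creature's type.
; Switching groups or removing a dead creature refreshes the HUD council, with deaths first advancing selection to the next creature.
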(event `self.ReceiveBeginPlay`
  (bind _outactors (`GameplayStatics.GetAllActorsOfClass` "/Game/Blueprints/Creatures/Wolf/Wolf.Wolf_C"))
  (set `self.Wolves` _outactors)
  (bind _outactors_2 (`GameplayStatics.GetAllActorsOfClass` "/Game/Blueprints/Creatures/Pig/Pig.Pig_C"))
  (set `self.Pigs` _outactors_2)
  (bind _outactors_3 (`GameplayStatics.GetAllActorsOfClass` "/Game/Blueprints/Creatures/Crocodile/Crocodile.Crocodile_C"))
  (set `self.Crocs` _outactors_3)
  (`KismetSystemLibrary.Delay` 0.2)
  (`self.SetOriginalCreature`)
  (`self.SetCreatureJobs`)
  (`self.SetCouncilPositions` (`self.Wolves`)))

(event `SetCreatureJobs`
  (for (_array_element _array_index) (`self.Wolves`)
    (`/Game/Blueprints/Creatures/CreatureBase.SetCreatureJob` _array_element (cast `/Game/Blueprints/Creatures/CreatureJobEnum` (`KismetMathLibrary.Conv_IntToByte` _array_index)))
    (for (_array_element_2 _array_index_2) (`self.Pigs`)
      (`/Game/Blueprints/Creatures/CreatureBase.SetCreatureJob` _array_element_2 (cast `/Game/Blueprints/Creatures/CreatureJobEnum` (`KismetMathLibrary.Conv_IntToByte` _array_index_2)))
      (for (_array_element_3 _array_index_3) (`self.Crocs`)
        (`/Game/Blueprints/Creatures/CreatureBase.SetCreatureJob` _array_element_3 (cast `/Game/Blueprints/Creatures/CreatureJobEnum` (`KismetMathLibrary.Conv_IntToByte` _array_index_3)))))))

(fn `GetNextCroc`
  (params (CurrentCroc :type "/Game/Blueprints/Creatures/Crocodile/Crocodile Object Reference"))
  (bind _crocs (`self.Crocs`))
  (bind _returnvalue (+ (`KismetArrayLibrary.Array_Find` _crocs CurrentCroc) 1))
  (if (< _returnvalue (`KismetArrayLibrary.Array_Length` _crocs))
    (set `self.SelectedCreature` (`|GetArrayItem` _crocs _returnvalue))
    (else
      (set `self.SelectedCreature` (`|GetArrayItem` _crocs)))))

(fn `GetNextPig`
  (params (CurrentPig :type "/Game/Blueprints/Creatures/Pig/Pig Object Reference"))
  (bind _pigs (`self.Pigs`))
  (bind _returnvalue (+ (`KismetArrayLibrary.Array_Find` _pigs CurrentPig) 1))
  (if (< _returnvalue (`KismetArrayLibrary.Array_Length` _pigs))
    (set `self.SelectedCreature` (`|GetArrayItem` _pigs _returnvalue))
    (else
      (set `self.SelectedCreature` (`|GetArrayItem` _pigs)))))

(fn `GetNextWolf`
  (params (CurrentWolf :type "/Game/Blueprints/Creatures/Wolf/Wolf Object Reference"))
  (bind _wolves (`self.Wolves`))
  (bind _returnvalue (+ (`KismetArrayLibrary.Array_Find` _wolves CurrentWolf) 1))
  (if (< _returnvalue (`KismetArrayLibrary.Array_Length` _wolves))
    (set `self.SelectedCreature` (`|GetArrayItem` _wolves _returnvalue))
    (else
      (set `self.SelectedCreature` (`|GetArrayItem` _wolves)))))

(fn `GetPreviousCroc`
  (params (CurrentCroc :type "/Game/Blueprints/Creatures/Crocodile/Crocodile Object Reference"))
  (bind _crocs (`self.Crocs`))
  (bind _returnvalue (- (`KismetArrayLibrary.Array_Find` _crocs CurrentCroc) 1))
  (if (> _returnvalue -1)
    (set `self.SelectedCreature` (`|GetArrayItem` _crocs _returnvalue))
    (else
      (set `self.SelectedCreature` (`|GetArrayItem` _crocs (- (`KismetArrayLibrary.Array_Length` _crocs) 1))))))

(fn `GetPreviousPig`
  (params (CurrentPig :type "/Game/Blueprints/Creatures/Pig/Pig Object Reference"))
  (bind _pigs (`self.Pigs`))
  (bind _returnvalue (- (`KismetArrayLibrary.Array_Find` _pigs CurrentPig) 1))
  (if (> _returnvalue -1)
    (set `self.SelectedCreature` (`|GetArrayItem` _pigs _returnvalue))
    (else
      (set `self.SelectedCreature` (`|GetArrayItem` _pigs (- (`KismetArrayLibrary.Array_Length` _pigs) 1))))))

(fn `GetPreviousWolf`
  (params (CurrentWolf :type "/Game/Blueprints/Creatures/Wolf/Wolf Object Reference"))
  (bind _wolves (`self.Wolves`))
  (bind _returnvalue (- (`KismetArrayLibrary.Array_Find` _wolves CurrentWolf) 1))
  (if (> _returnvalue -1)
    (set `self.SelectedCreature` (`|GetArrayItem` _wolves _returnvalue))
    (else
      (set `self.SelectedCreature` (`|GetArrayItem` _wolves (- (`KismetArrayLibrary.Array_Length` _wolves) 1))))))

(fn `GoToNextCreature`
  (params (CurrentCreature :type "/Game/Blueprints/Creatures/CreatureBase Object Reference"))
  (switch `/Game/Blueprints/Creatures/CreatureTypes` (`/Game/Blueprints/Creatures/CreatureBase.CreatureType` CurrentCreature)
    (:`NewEnumerator0`
      (bind _aswolf (cast `/Game/Blueprints/Creatures/Wolf/Wolf` CurrentCreature))
      (`self.GetNextWolf` _aswolf))
    (:`NewEnumerator1`
      (bind _ascrocodile (cast `/Game/Blueprints/Creatures/Crocodile/Crocodile` CurrentCreature))
      (`self.GetNextCroc` _ascrocodile))
    (:`NewEnumerator10`
      (bind _aspig (cast `/Game/Blueprints/Creatures/Pig/Pig` CurrentCreature))
      (`self.GetNextPig` _aspig)))
  (`/Game/Blueprints/Creatures/CreatureBase.SelectCreature` (`self.SelectedCreature`)))

(fn `GoToPreviousCreature`
  (params (CurrentCreature :type "/Game/Blueprints/Creatures/CreatureBase Object Reference"))
  (switch `/Game/Blueprints/Creatures/CreatureTypes` (`/Game/Blueprints/Creatures/CreatureBase.CreatureType` CurrentCreature)
    (:`NewEnumerator0`
      (bind _aswolf (cast `/Game/Blueprints/Creatures/Wolf/Wolf` CurrentCreature))
      (`self.GetPreviousWolf` _aswolf))
    (:`NewEnumerator1`
      (bind _ascrocodile (cast `/Game/Blueprints/Creatures/Crocodile/Crocodile` CurrentCreature))
      (`self.GetPreviousCroc` _ascrocodile))
    (:`NewEnumerator10`
      (bind _aspig (cast `/Game/Blueprints/Creatures/Pig/Pig` CurrentCreature))
      (`self.GetPreviousPig` _aspig)))
  (`/Game/Blueprints/Creatures/CreatureBase.SelectCreature` (`self.SelectedCreature`)))

(fn `RemoveDeadCreature`
  (params (DeadCreature :type "/Game/Blueprints/Creatures/CreatureBase Object Reference"))
  (bind _wolves (`self.Wolves`))
  (bind _pigs (`self.Pigs`))
  (bind _crocs (`self.Crocs`))
  (bind _astbchud (cast `/Game/Blueprints/Widgets/TBCHud` (`PlayerController.GetHUD` (`GameplayStatics.GetPlayerController` 0))))
  (bind _aswolf (cast `/Game/Blueprints/Creatures/Wolf/Wolf` DeadCreature)
    (:`then`
      (`self.GoToNextCreature` _aswolf)
      (`KismetArrayLibrary.Array_RemoveItem` _wolves _aswolf)
      (bind _ui_ref (`/Game/Blueprints/Widgets/TBCHud.UI Ref` _astbchud))
      (`/Game/Blueprints/Widgets/TBCUI.UpdateCouncil` _ui_ref _wolves))
    (:`CastFailed`
      (bind _aspig (cast `/Game/Blueprints/Creatures/Pig/Pig` DeadCreature)
        (:`then`
          (`self.GoToNextCreature` _aspig)
          (`KismetArrayLibrary.Array_RemoveItem` _pigs _aspig)
          (`/Game/Blueprints/Widgets/TBCUI.UpdateCouncil` _ui_ref _pigs))
        (:`CastFailed`
          (bind _ascrocodile (cast `/Game/Blueprints/Creatures/Crocodile/Crocodile` DeadCreature))
          (`self.GoToNextCreature` _ascrocodile)
          (`KismetArrayLibrary.Array_RemoveItem` _crocs _ascrocodile)
          (`/Game/Blueprints/Widgets/TBCUI.UpdateCouncil` _ui_ref _crocs))))))

(fn `SetCouncilPositions`
  (params (Creatures :type "Array of /Game/Blueprints/Creatures/CreatureBase Object Reference"))
  (bind _astbchud (cast `/Game/Blueprints/Widgets/TBCHud` (`PlayerController.GetHUD` (`GameplayStatics.GetPlayerController` 0))))
  (`/Game/Blueprints/Widgets/TBCUI.UpdateCouncil` (`/Game/Blueprints/Widgets/TBCHud.UI Ref` _astbchud) Creatures))

(fn `SetCrocs`
  (bind _crocs (`self.Crocs`))
  (`self.SetCouncilPositions` _crocs)
  (`/Game/Blueprints/Creatures/CreatureBase.SelectCreature` (`|GetArrayItem` _crocs)))

(fn `SetOriginalCreature`
  (bind _wolves (`self.Wolves`))
  (bind _output (`|GetArrayItem` _wolves))
  (`self.SetCouncilPositions` _wolves)
  (`/Game/Blueprints/Creatures/CreatureBase.SelectCreature` _output)
  (`self.SetSelectedCreature` _output))

(fn `SetPigs`
  (bind _pigs (`self.Pigs`))
  (`self.SetCouncilPositions` _pigs)
  (`/Game/Blueprints/Creatures/CreatureBase.SelectCreature` (`|GetArrayItem` _pigs)))

(fn `SetSelectedCreature`
  (params (Creature :type "/Game/Blueprints/Creatures/CreatureBase Object Reference"))
  (set `self.SelectedCreature` Creature))

(fn `SetWolves`
  (bind _wolves (`self.Wolves`))
  (`self.SetCouncilPositions` _wolves)
  (`/Game/Blueprints/Creatures/CreatureBase.SelectCreature` (`|GetArrayItem` _wolves)))

(fn `UserConstructionScript`)