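; Player camera actor that makes itself the view target on BeginPlay and registers with the TBCPlayerController.
; ZoomCamera toggles between zoomed-out and zoomed-in by moving the root component between BackPos and ForwardPos, rather than changing FOV.
; ZoomIn and ZoomOut timelines drive the location lerp, while a CameraState enum tracks transitions and ignores zoom calls mid-move.
; The CameraZoom function is an empty stub.
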(event `self.ReceiveBeginPlay`
  (bind _returnvalue (`GameplayStatics.GetPlayerController` 0))
  ;[1 1 1] setting this camera to active player camera
  (set `self.bFindCameraComponentWhenViewTarget` true)
  (`PlayerController.SetViewTargetWithBlend` _returnvalue self 0.0 "VTBlend_Cubic" 0.0 false)
  (bind _astbcplayer_controller (cast `/Game/Blueprints/TBCPlayerController` _returnvalue))
  (`/Game/Blueprints/TBCPlayerController.SetPlayerCamera` _astbcplayer_controller self))

(event `ZoomCamera`
  ;[1 1 1] Camera Zoom Functionality
  (switch `/Game/Blueprints/CameraState` (`self.CameraState`)
    (:`NewEnumerator0`
      (set `self.CameraState` "NewEnumerator4")
      (bind (_direction _zoominpercent) (`Timeline|ZoomIn` :!via `PlayFromStart`)
        (:`Update`
          (`SceneComponent.K2_SetWorldLocation` (`self.RootComponent`) (`KismetMathLibrary.VLerp` (`self.BackPos`) (`self.ForwardPos`) _zoominpercent) false false))
        (:`Finished`
          (set `self.CameraState` "NewEnumerator2"))))
    (:`NewEnumerator2`
      (set `self.CameraState` "NewEnumerator1")
      (bind (_direction_2 _zoominpercent_2) (`Timeline|ZoomOut` :!via `PlayFromStart`)
        (:`Update`
          (`SceneComponent.K2_SetWorldLocation` (`self.RootComponent`) (`KismetMathLibrary.VLerp` (`self.ForwardPos`) (`self.BackPos`) _zoominpercent_2) false false))
        (:`Finished`
          (set `self.CameraState` "NewEnumerator0"))))))

(fn `CameraZoom`)

(fn `UserConstructionScript`)