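; CreatureBase is a base creature Blueprint that tracks mouse interaction with its Mesh in an enum status variable, MyStatus.
; The status starts in a default state at BeginPlay and returns to it when the cursor leaves.
; Hovering or releasing a click sets a second state, and clicking sets a third.
; Each mouse event prints the new status to screen as debug output.
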(event `self.ReceiveBeginPlay`
  (set `self.MyStatus` "NewEnumerator0"))

(event `self.Mesh.OnBeginCursorOver`
  (params (TouchedComponent :type "PrimitiveComponent Object Reference"))
  (bind _output_get (set `self.MyStatus` "NewEnumerator1"))
  (`KismetSystemLibrary.PrintString` (`|GetEnumeratorNameAsString` _output_get)))

(event `self.Mesh.OnEndCursorOver`
  (params (TouchedComponent :type "PrimitiveComponent Object Reference"))
  (bind _output_get (set `self.MyStatus` "NewEnumerator0"))
  (`KismetSystemLibrary.PrintString` (`|GetEnumeratorNameAsString` _output_get)))

(event `self.Mesh.OnClicked`
  (params (TouchedComponent :type "PrimitiveComponent Object Reference") (ButtonPressed :type "Key Structure"))
  (bind _output_get (set `self.MyStatus` "NewEnumerator2"))
  (`KismetSystemLibrary.PrintString` (`|GetEnumeratorNameAsString` _output_get)))

(event `self.Mesh.OnReleased`
  (params (TouchedComponent :type "PrimitiveComponent Object Reference") (ButtonReleased :type "Key Structure"))
  (bind _output_get (set `self.MyStatus` "NewEnumerator1"))
  (`KismetSystemLibrary.PrintString` (`|GetEnumeratorNameAsString` _output_get)))

(fn `UserConstructionScript`)