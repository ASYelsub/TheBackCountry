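; BP_WeatherSystem is a day-night cycle actor that rotates a referenced Sun over a configurable day length in minutes.
; Tick advances a 24-hour clock, wrapping past 24, and maps it through DayLengthCurve to the Sun's pitch.
; The construction script snaps the actor to the world origin location and previews the Sun pitch if Sun, SkyLight, SkyAtmosphere and Fog are valid, using a different yaw than Tick.
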(event `self.ReceiveBeginPlay`
  (set `self.OneHour` (/ (* (`self.DayLengthInMinutes`) 60.0) 24.0)))

(event `self.ReceiveTick`
  (params (DeltaSeconds :type "Float (single-precision)"))
  (bind _returnvalue (+ (`KismetMathLibrary.SafeDivide` DeltaSeconds (`self.OneHour`)) (`self.CurrentTime`)))
  (if (> _returnvalue 0.0)
    (if (<= _returnvalue 24.0)
      (set `self.CurrentTime` _returnvalue)
      (else
        (set `self.CurrentTime` (`KismetMathLibrary.Abs` (- 24.0 _returnvalue)))))
    (`self.K2_SetActorRotation` (`self.Sun`) (`KismetMathLibrary.MakeRotator` 0.0 (`CurveFloat.GetFloatValue` (`self.DayLengthCurve`) (`self.CurrentTime`)) -90.0) false)))

(fn `UserConstructionScript`
  (`self.K2_SetActorLocation` (`KismetMathLibrary.Conv_IntVectorToVector` (`GameplayStatics.GetWorldOriginLocation`)))
  (`/Engine/EditorBlueprintResources/StandardMacros.IsValid` (`self.Sun`)
    (:`Is Valid`
      (`/Engine/EditorBlueprintResources/StandardMacros.IsValid` (`self.SkyLight`)
        (:`Is Valid`
          (`/Engine/EditorBlueprintResources/StandardMacros.IsValid` (`self.SkyAtmosphere`)
            (:`Is Valid`
              (`/Engine/EditorBlueprintResources/StandardMacros.IsValid` (`self.Fog`)
                (:`Is Valid`
                  (`self.K2_SetActorRotation` (`self.Sun`) (`KismetMathLibrary.MakeRotator` 0.0 (`CurveFloat.GetFloatValue` (`self.DayLengthCurve`) (`self.CurrentTime`))) false))))))))))